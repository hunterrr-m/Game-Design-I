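; Follower pawn Blueprint that uses AI movement to trail the first player character.
; StartFollow calls MoveTo, which runs AIMoveTo toward the player with a two-meter acceptance radius.
; Both success and failure print a debug message, wait a second, then re-issue MoveTo while IsFollowing is true, forming a self-repeating follow loop without Tick.
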(event Custom|MoveTo
  (AI|AIMoveTo self "0, 0, 0" (Game|GetPlayerCharacter 0) 2e+02 false ; Move to player location, and stop 2 meters away.
    (:OnSuccess
      (Development|PrintString "Success! Got to player destination." true true "(R=0.081878,G=1.000000,B=0.000000,A=1.000000)"))
    (:OnFail
      (Development|PrintString "Failed to get to player destination." true true "(R=1.000000,G=0.000000,B=0.031016,A=1.000000)" 5.0)))
  (Utilities|FlowControl|Delay 1.0)
  (if (Variables|Default|GetIsFollowing)
    (CallFunction|Moveto)))

(event Custom|StartFollow
  (CallFunction|Moveto))

(fn ConstructionScript)