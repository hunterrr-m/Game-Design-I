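; Lap-timing finish frame that shows a running lap time and reports each lap when the custom third-person character passes through it.
; On BeginPlay it creates the W_InterfaceTimer widget and starts a self-calling Delay loop that refreshes the widget text and a debug print every tenth of a second.
; Overlapping the Box prints the real seconds since the last timestamp, then resets it to start the next lap.
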(event OnComponentBeginOverlap(Box)
  (params (OverlappedComponent :type Primitive%20Component%20Object%20Reference) (OtherActor :type Actor%20Object%20Reference) (OtherComp :type Primitive%20Component%20Object%20Reference) (OtherBodyIndex :type Integer) (bFromSweep :type Boolean) (SweepResult :type Hit%20Result%20Structure%20%28by%20ref%29))
  ;[0.2544 1 0] Calling your current lap when running through frame.
  (Utilities|Casting|CastToBP_ThirdPersonCharacterCustom OtherActor)
  (Development|PrintString (Utilities|String|Append "That lap took " (Utilities|String|ToString(Text) (Utilities|Text|ToText(Float) (- (Utilities|Time|GetRealTimeSeconds) (Variables|Default|GetLastTimestamp)) "HalfToEven" false true 1 324 0 1)) " seconds."))
  (Variables|Default|SetLastTimestamp (Utilities|Time|GetRealTimeSeconds)))

(event Custom|OnScreenTimer
  (bind _returnvalue (Utilities|Time|GetRealTimeSeconds))
  (bind _lasttimestamp (Variables|Default|GetLastTimestamp))
  (bind _returnvalue_2 (- _returnvalue _lasttimestamp))
  (bind _returnvalue_3 (Utilities|Text|ToText(Float) _returnvalue_2 "HalfToEven" false true 1 324 0 1))
  (bind _returnvalue_4 (Utilities|String|ToString(Text) _returnvalue_3))
  (bind _returnvalue_5 (Utilities|String|Append "Current lap: " _returnvalue_4 " seconds."))
  ;[0.07843 0.3373 1] Setting the on-screen timer every .1 second(s)
  (Development|PrintString _returnvalue_5 true true "(R=0.000000,G=0.660000,B=1.000000,A=1.000000)" 0.1)
  (Variables|/Script/UMG.TextBlock|SetText (Variables|/Game/Widgets/W_InterfaceTimer.W_InterfaceTimer_C|GetCurrentTimeText (Variables|Default|GetW%20Timer%20Widget)) (Utilities|Text|ToText(String) _returnvalue_5))
  (Utilities|FlowControl|Delay 0.1)
  (CallFunction|OnScreenTimer))

(event EventBeginPlay
  ;[0.07843 0.3373 1] Adding on-screen timer to viewport.
  (bind _returnvalue (UserInterface|CreateWidget "/Game/Widgets/W_InterfaceTimer.W_InterfaceTimer_C"))
  (bind _output_get (Variables|Default|SetW%20Timer%20Widget _returnvalue))
  (UserInterface|Viewport|AddtoViewport _output_get 0)
  (CallFunction|OnScreenTimer))

(event Collision|EventActorBeginOverlap
  (params (OtherActor :type Actor%20Object%20Reference)))

(event EventTick
  (params (DeltaSeconds :type Float%20%28single-precision%29)))

(fn ConstructionScript)