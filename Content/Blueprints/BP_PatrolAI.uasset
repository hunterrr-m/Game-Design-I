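; Patrol AI character that walks between tagged patrol point actors in an endless loop.
; On BeginPlay it gathers and shuffles the tagged points, randomizes its walk speed, and starts moving.
; AI MoveTo advances through the array after a short delay on success or failure, reshuffling after each full pass.
; A separate MoveTo event repeatedly follows the player but is not called within this graph.
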(event Custom|GoToPatrolPoint
  ;[1 0.7744 0] Move Patrol AI to first patrol point in array, then continue down the array. Start again when finished.
  (AI|AIMoveTo self (Transformation|GetActorLocation (Utilities|Array|Get(acopy) (stale EventBeginPlay _outactors) (Variables|Default|GetCurrentPatrolPoint))) 0 2e+02 false ; Move to player location, and stop 2 meters away.
    (:OnSuccess
      (Development|PrintString "Success! Got to patrol point." true true "(R=0.081878,G=1.000000,B=0.000000,A=1.000000)"))
    (:OnFail
      (Development|PrintString "Failed to get to next patrol point." true true "(R=1.000000,G=0.000000,B=0.031016,A=1.000000)" 5.0)))
  (bind _result (Math|Integer|IncrementInt (Variables|Default|GetCurrentPatrolPoint))
    (:%20%20
      (if (>= _result (Utilities|Array|Length (stale EventBeginPlay _outactors)))
        (Variables|Default|SetCurrentPatrolPoint 0)
        (Utilities|Array|Shuffle (stale EventBeginPlay _outactors)))
      (Utilities|FlowControl|Delay 1.0)
      (CallFunction|GotoPatrolPoint))))

(event Custom|MoveTo
  (AI|AIMoveTo self "0, 0, 0" (Game|GetPlayerCharacter 0) 2e+02 false ; Move to player location, and stop 2 meters away.
    (:OnSuccess
      (Development|PrintString "Success! Got to player destination." true true "(R=0.081878,G=1.000000,B=0.000000,A=1.000000)"))
    (:OnFail
      (Development|PrintString "Failed to get to player destination." true true "(R=1.000000,G=0.000000,B=0.031016,A=1.000000)" 5.0)))
  (Utilities|FlowControl|Delay 1.0)
  (CallFunction|Moveto))

(event EventBeginPlay
  ;[1 0.445 0] Get all patrol points, set random walk speed, and call 'GoToPatrolPoint'
  (bind _outactors (Actor|GetAllActorsOfClasswithTag "/Script/Engine.Actor" (Variables|Default|GetPatrolPointTag)))
  (Development|PrintString (Utilities|String|Append "There are " (Utilities|String|ToString(Integer) (Utilities|Array|Length _outactors)) " patrol points.") true true "(R=0.047576,G=0.000000,B=1.000000,A=1.000000)" 1e+01)
  (Utilities|Array|Shuffle _outactors)
  (Variables|/Script/Engine.CharacterMovementComponent|SetMaxWalkSpeed (Variables|Character|GetCharacterMovement) (Math|Conversions|ToFloat(Integer) (* (Math|Random|RandomIntegerinRange 8 12) 25)))
  (CallFunction|GotoPatrolPoint))

(fn ConstructionScript)