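; Level-exit trigger that sends the player to DestinationLvl when a BP_ThirdPersonCharacterCustom overlaps its Trigger component.
; It fades camera and audio out, waits for the fade, then opens the level by object reference, or prints a message if the destination is invalid.
; The fade-in and the character's level name and number updates are called right after the open call, on the current level's camera manager and character.
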(event OnComponentBeginOverlap(Trigger)
  (params (OverlappedComponent :type Primitive%20Component%20Object%20Reference) (OtherActor :type Actor%20Object%20Reference) (OtherComp :type Primitive%20Component%20Object%20Reference) (OtherBodyIndex :type Integer) (bFromSweep :type Boolean) (SweepResult :type Hit%20Result%20Structure%20%28by%20ref%29))
  (bind _returnvalue (Game|GetPlayerCameraManager 0))
  ;[0.05559 1 0.9662] Get current level.
  (bind _asbp_third_person_character_custom (Utilities|Casting|CastToBP_ThirdPersonCharacterCustom OtherActor))
  (bind _destinationlvl (Variables|Default|GetDestinationLvl)
    (:then
      ;[0.449 0.449 0.449] Fade to black, load next level, fade back into view.
      (CameraFades|StartCameraFade :self _returnvalue :ToAlpha 1.0 :Duration 0.8 :bShouldFadeAudio true :bHoldWhenFinished true)
      (Utilities|FlowControl|Delay 0.8)
      (Game|OpenLevel(byObjectReference) _destinationlvl)
      (CameraFades|StartCameraFade :self _returnvalue :FromAlpha 1.0 :Duration 0.8 :bShouldFadeAudio true :bHoldWhenFinished true)
      ;[1 0.01124 0.6965] Update current level number and level name.
      (Default|UpdateLevelName _asbp_third_person_character_custom (Variables|Default|GetNewLevelName))
      (Default|UpdateLevelNumber _asbp_third_person_character_custom (Variables|Default|GetNewLevelNum)))
    (:else
      (Development|PrintString "No valid destination." true true "(R=1.000000,G=0.000000,B=0.062690,A=1.000000)" 5.0))))

(event EventBeginPlay)

(event Collision|EventActorBeginOverlap
  (params (OtherActor :type Actor%20Object%20Reference)))

(event EventTick
  (params (DeltaSeconds :type Float%20%28single-precision%29)))

(fn ConstructionScript)