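; BP_DialogueCircle is a dialogue trigger actor that sends a dialogue update to the player character when entered.
; Each Tick it turns horizontally to face the player pawn, flattening the direction vector so it only yaws.
; The first overlap of its Trigger by a BP_ThirdPersonCharacterCustom calls UpdateDialogue on that character with DialogueNum.
; A DoOnce with no reset wired keeps it from firing again.
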(event OnComponentBeginOverlap(Trigger)
  (params (OverlappedComponent :type Primitive%20Component%20Object%20Reference) (OtherActor :type Actor%20Object%20Reference) (OtherComp :type Primitive%20Component%20Object%20Reference) (OtherBodyIndex :type Integer) (bFromSweep :type Boolean) (SweepResult :type Hit%20Result%20Structure%20%28by%20ref%29))
  (bind _asbp_third_person_character_custom (Utilities|Casting|CastToBP_ThirdPersonCharacterCustom OtherActor))
  (Utilities|FlowControl|DoOnce false
    (:Completed
      (Default|UpdateDialogue _asbp_third_person_character_custom (Variables|Default|GetDialogueNum)))))

(event EventBeginPlay)

(event Collision|EventActorBeginOverlap
  (params (OtherActor :type Actor%20Object%20Reference)))

(event EventTick
  (params (DeltaSeconds :type Float%20%28single-precision%29))
  (Transformation|SetActorRotation (Math|Conversions|RotationFromXVector (Math|Vector|RotateVector (Math|Vector|Normalize (* (- (Transformation|GetActorLocation (Game|Player|GetPlayerPawn 0)) (Transformation|GetActorLocation)) "1.000000,1.000000,0.000000")) "0, 0, 0"))))

(fn ConstructionScript)